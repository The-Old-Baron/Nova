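; Player controller for Nova that creates the main HUD and connects the possessed character to the ALS camera.
; On possess, it caches the Nova character and passes it to the ALS player camera manager.
; Tick pushes the character's current and max oxygen and stamina to the HUD every frame.
; The debug-info interface function reports every debug option as disabled.
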(event EventBeginPlay
  (|CallParentFunction)
  (bind _returnvalue (UserInterface|CreateWidget "/Game/Nova/Blueprints/Widget/Widget_MainHUD.Widget_MainHUD_C"))
  (bind _output_get (Variables|Default|SetMainHud _returnvalue))
  (UserInterface|Viewport|AddtoViewport _output_get 0))

(event EventPossess
  (params (PossessedPawn :type Pawn%20Object%20Reference))
  (|CallParentFunction PossessedPawn)
  (bind _asbp_nova_character (Utilities|Casting|CastToBP_Nova_Character PossessedPawn))
  (bind _output_get (Variables|Default|SetNovaCharacter _asbp_nova_character))
  (bind _asals_player_camera_manager (Utilities|Casting|CastToALS_PlayerCameraManager (Variables|Default|GetPlayerCameraManager)))
  (Default|OnPossess _asals_player_camera_manager _output_get))

(event EventTick
  (params (DeltaSeconds :type Float%20%28single-precision%29))
  (bind _novacharacter (Variables|Default|GetNovaCharacter))
  (bind _mainhud (Variables|Default|GetMainHud))
  (|CallParentFunction DeltaSeconds)
  (Default|UpdateOxigen _mainhud (Variables|/Game/Nova/Blueprints/Core/BP_Nova_Character.BP_Nova_Character_C|GetMaxOxigen _novacharacter) (Variables|/Game/Nova/Blueprints/Core/BP_Nova_Character.BP_Nova_Character_C|GetCurrentOxigen _novacharacter))
  (Default|UpdateStamina _mainhud (Variables|/Game/Nova/Blueprints/Core/BP_Nova_Character.BP_Nova_Character_C|GetMaxStamina _novacharacter) (Variables|/Game/Nova/Blueprints/Core/BP_Nova_Character.BP_Nova_Character_C|GetCurrentStamina _novacharacter)))

(fn ConstructionScript
  (|CallParentFunction))

(fn BPIGetDebugInfo
  (return 0 false false false false false false false))