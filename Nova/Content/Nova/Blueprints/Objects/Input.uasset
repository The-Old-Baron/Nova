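; Interactable switch that toggles a circuit of lamps on and off.
; At BeginPlay it gathers BPI_Lamps actors whose circuit number equals their index in the search results, then switches them on regardless of IsOn.
; Each interaction flips IsOn, recolors the cube blue or red, and sends the matching on/off interface message to those lamps.
; The construction script sets the cube's color from IsOn.
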(event OnInteract(Interactable)
  (params (Interactor :type Interactor%20Component%20Object%20Reference) (Interactable :type Interactable%20Component%20Object%20Reference))
  (bind _output_get (Variables|Default|SetIsOn (not (Variables|Default|GetIsOn))))
  (if _output_get
    (CallFunction|On)
    (else
      (CallFunction|Off))))

(event EventBeginPlay
  (bind _outactors (Actor|GetAllActorswithInterface "/Game/Nova/Blueprints/Interface/BPI_Lamps.BPI_Lamps_C"))
  (for (_array_element _array_index) _outactors
    (bind _circuitcode (Class|BPILamps|GetCircuit(Message) _array_element))
    (if (== _circuitcode _array_index)
      (Utilities|Array|Add (Variables|Default|GetLampsOnCircuit) _array_element)))
  (for _array_element_2 (Variables|Default|GetLampsOnCircuit)
    (Class|BPILamps|Seton(Message) _array_element_2)))

(event Collision|EventActorBeginOverlap
  (params (OtherActor :type Actor%20Object%20Reference)))

(event EventTick
  (params (DeltaSeconds :type Float%20%28single-precision%29)))

(fn ConstructionScript
  (if (Variables|Default|GetIsOn)
    (Rendering|Material|SetMaterial (Variables|Default|GetCube) 0 "/Game/Nova/Material/Placeholder/BlueDefault.BlueDefault")
    (else
      (Rendering|Material|SetMaterial (Variables|Default|GetCube) 0 "/Game/Nova/Material/Placeholder/RedDefault.RedDefault"))))

(fn On
  (Rendering|Material|SetMaterial (Variables|Default|GetCube) 0 "/Game/Nova/Material/Placeholder/BlueDefault.BlueDefault")
  (for _array_element (Variables|Default|GetLampsOnCircuit)
    (Class|BPILamps|Seton(Message) _array_element)))

(fn Off
  (Rendering|Material|SetMaterial (Variables|Default|GetCube) 0 "/Game/Nova/Material/Placeholder/RedDefault.RedDefault")
  (for _array_element (Variables|Default|GetLampsOnCircuit)
    (Class|BPILamps|SetOff(Message) _array_element)))