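; Switchable lamp actor that tracks an on/off state and exposes its Circuit value through a getter.
; On and Off set IsOn and swap the lamp mesh material, and ToggleState picks between them.
; SetOff chains through server and client events, each reapplying Off, while Seton has no such chain.
; The set events print the new state, and the construction script and default events are empty.
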(event Custom|SERVER_Set%20Off
  (CallFunction|Off)
  (Development|PrintText "Off")
  (CallFunction|CLIENTSetOff))

(event Custom|CLIENT_Set%20Off
  (CallFunction|Off)
  (Development|PrintText "Off"))

(event EventBeginPlay)

(event Collision|EventActorBeginOverlap
  (params (OtherActor :type Actor%20Object%20Reference)))

(event EventTick
  (params (DeltaSeconds :type Float%20%28single-precision%29)))

(event EventToggleState
  (params (CircuitCode :type Integer))
  (if (not (Variables|Default|GetIsOn))
    (CallFunction|On)
    (else
      (CallFunction|Off))))

(event EventSeton
  (params (CircuitCode :type Integer))
  (CallFunction|On)
  (Development|PrintText "On"))

(event EventSetOff
  (params (CircuitCode :type Integer))
  (CallFunction|Off)
  (Development|PrintText "Off")
  (CallFunction|SERVERSetOff))

(fn ConstructionScript)

(fn On
  (Variables|Default|SetIsOn true)
  (Rendering|Material|SetMaterial (Variables|Default|GetSM_Lamp01) 0 (Variables|Default|GetMaterial_On)))

(fn Off
  (Variables|Default|SetIsOn false)
  (Rendering|Material|SetMaterial (Variables|Default|GetSM_Lamp01) 0 (Variables|Default|GetMaterial_Off)))

(fn GetCircuit
  (return (Variables|Default|GetCircuit)))